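; AI controller for BP_AIChar that makes it wander continuously between random target points.
; On BeginPlay it caches the pawn and picks a reachable point within a radius.
; Tick draws a debug box at the target and re-issues AI MoveTo, choosing a new point on success.
; Tick also runs CheckActorLocation, which retargets inside a bounding box whenever the pawn leaves the X/Y limits.
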(event `self.ReceiveBeginPlay`
  (bind _asbp_aichar (cast `/Game/10dot7HW/Blueprints/AI/BP_AIChar` (`self.K2_GetPawn`)))
  (set `self.ControlledPawn` _asbp_aichar)
  (`self.SetRandomTargetPoint`))

(event `self.ReceiveTick`
  (params (DeltaSeconds :type "Float (single-precision)"))
  (`|ExecutionSequence`
    (:`then_0`
      (`KismetSystemLibrary.DrawDebugBox` (`self.TargetPoint`) (5.0 5.0 5.0) (struct :`B` 1.0 :`A` 1.0) (struct) 0.0 3.0))
    (:`then_1`
      (`|AIMoveTo` null (`self.TargetPoint`) null
        (:`OnSuccess`
          (`self.SetRandomTargetPoint`))))
    (:`then_2`
      (`self.CheckActorLocation`))))

(event `SetRandomTargetPointInBox`
  (set `self.TargetPoint` (`KismetMathLibrary.RandomPointInBoundingBox_Box` (`KismetMathLibrary.MakeBox` (`KismetMathLibrary.MakeVector` (`self.MinX`) (`self.MinY`) 10.0) (`KismetMathLibrary.MakeVector` (`self.MaxX`) (`self.MaxY`) 10.0)))))

(event `SetRandomTargetPoint`
  (set `self.TargetPoint` (`NavigationSystemV1.K2_GetRandomReachablePointInRadius` (`self.K2_GetActorLocation` (`self.ControlledPawn`)) 5000.0 null null)))

(fn `CheckActorLocation`
  (bind (_returnvalue_x _returnvalue_y) (`KismetMathLibrary.BreakVector` (`self.K2_GetActorLocation` (`self.ControlledPawn`))))
  (if (< _returnvalue_x (`self.MinX`))
    (`self.SetRandomTargetPointInBox`)
    (elif (> _returnvalue_x (`self.MaxX`))
      (`self.SetRandomTargetPointInBox`)
      (elif (< _returnvalue_y (`self.MinY`))
        (`self.SetRandomTargetPointInBox`)
        (elif (> _returnvalue_y (`self.MaxY`))
          (`self.SetRandomTargetPointInBox`))))))

(fn `UserConstructionScript`)